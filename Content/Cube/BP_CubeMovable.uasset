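; BP_CubeMovable is a cube that puts the third-person player into a slowed pushing state while they overlap its Collision component.
; Overlap events toggle a flag that gates Tick, which sets the player's IsPushing and lowers MaxWalkSpeed only when X, Y and Z velocity are all non-zero.
; Zero Z velocity clears both, while leaving the overlap restores speed but not IsPushing.
; The graph never moves the cube itself.
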(event `self.ReceiveBeginPlay`
  (bind _asbp_third_person_character (cast `/Game/ThirdPerson/Blueprints/BP_ThirdPersonCharacter` (`GameplayStatics.GetPlayerCharacter` 0)))
  (set `self.PlayerRef` _asbp_third_person_character))

(event `self.Collision.OnComponentBeginOverlap`
  (params (OverlappedComponent :type "PrimitiveComponent Object Reference") (OtherActor :type "Actor Object Reference") (OtherComp :type "PrimitiveComponent Object Reference") (OtherBodyIndex :type Integer) (bFromSweep :type Boolean) (SweepResult :type "HitResult Structure (by ref)"))
  (if (== OtherActor (`self.PlayerRef`))
    (set `self.Tick` true)
    (else
      (set `self.Tick` false))))

(event `self.Collision.OnComponentEndOverlap`
  (params (OverlappedComponent :type "PrimitiveComponent Object Reference") (OtherActor :type "Actor Object Reference") (OtherComp :type "PrimitiveComponent Object Reference") (OtherBodyIndex :type Integer))
  (if (== OtherActor (`self.PlayerRef`))
    (set `self.Tick` false)
    (set `CharacterMovementComponent.MaxWalkSpeed` 600.0 (`Character.CharacterMovement` (`self.PlayerRef`)))))

(event `self.ReceiveTick`
  (params (DeltaSeconds :type "Float (single-precision)"))
  (bind _playerref (`self.PlayerRef`))
  (bind _charactermovement (`Character.CharacterMovement` _playerref))
  (if (`self.Tick`)
    (if (!= (.x (`MovementComponent.Velocity` (`Character.CharacterMovement` (`self.PlayerRef`)))) 0.0)
      (if (!= (.y (`MovementComponent.Velocity` (`Character.CharacterMovement` (`self.PlayerRef`)))) 0.0)
        (if (!= (.z (`MovementComponent.Velocity` (`Character.CharacterMovement` (`self.PlayerRef`)))) 0.0)
          (set `/Game/ThirdPerson/Blueprints/BP_ThirdPersonCharacter.IsPushing` true _playerref)
          (set `CharacterMovementComponent.MaxWalkSpeed` 100.0 _charactermovement)
          (else
            (set `/Game/ThirdPerson/Blueprints/BP_ThirdPersonCharacter.IsPushing` false _playerref)
            (set `CharacterMovementComponent.MaxWalkSpeed` 600.0 _charactermovement)))))))

(fn `UserConstructionScript`)